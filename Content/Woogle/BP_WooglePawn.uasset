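; BP_WooglePawn is a pawn that sets up positional VOIP voice chat for its player.
; On BeginPlay it adds a VOIP talker, then retries on a short delay until PlayerState is valid to register it.
; It sets the mic threshold and attaches attenuated voice to the root component.
; The locally controlled pawn also enables voice loopback and prints a confirmation; ToggleSpeaking command nodes are left unconnected.
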(event `self.ReceiveBeginPlay`
  (bind _returnvalue (`AddComponent|NODE_AddVOIPTalker-0`))
  (set `self.VOIPRef` _returnvalue)
  (`/Engine/EditorBlueprintResources/StandardMacros.IsValid` (`self.PlayerState`) :!label _label
    (:`Is Valid`
      (`VOIPTalker.RegisterWithPlayerState` (`self.VOIPRef`) (`self.PlayerState`))
      (`VOIPStatics.SetMicThreshold` -1.0)
      (set `VOIPTalker.Settings` (make `VoiceSettings` (`self.RootComponent`) "/Game/Woogle/SA_VoiceChat.SA_VoiceChat") (`self.VOIPRef`))
      (if (`self.IsLocallyControlled`)
        (`KismetSystemLibrary.ExecuteConsoleCommand` "OSS.VoiceLoopback 1" null)
        (`KismetSystemLibrary.PrintString` "Voice chat Enabled!")))
    (:`Is Not Valid`
      (`KismetSystemLibrary.Delay` 0.2)
      (goto _label))))

(fn `UserConstructionScript`)