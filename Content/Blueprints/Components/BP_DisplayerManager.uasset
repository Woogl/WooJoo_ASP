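; BP_DisplayerManager manages a single text displayer actor that it shows at a location, edits or deletes.
; ShowDisplayer, EditDisplayer and DeleteDisplayer use the ShouldReplicates flag to pick Server or Client events, with show and edit also playing a 2D sound, via Multi_PlaySound when replicated.
; GetExistingDisplayer returns the cached actor or finds one by class, so showing moves and retexts an existing displayer, spawning only when none exists.
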(event `Server_ShowDisplayer`
  (params (InText :type Text) (DisplayerLocation :type "Vector Structure"))
  (bind _existingdisplayer (`self.GetExistingDisplayer`))
  (`/Engine/EditorBlueprintResources/StandardMacros.IsValid` _existingdisplayer
    (:`Is Valid`
      (`Actor.K2_SetActorLocation` _existingdisplayer DisplayerLocation false true)
      (message `/Game/Blueprints/Interfaces/BPI_Displayer.ChangeText` _existingdisplayer InText))
    (:`Is Not Valid`
      (bind _returnvalue (`|SpawnActorFromClass` (`self.DisplayerClass`) (`KismetMathLibrary.MakeTransform` DisplayerLocation) "AlwaysSpawn" "OverrideRootScale" null (`self.ShouldReplicates`) (`GameplayStatics.GetPlayerPawn` 0)))
      (bind _output_get (set `self.DisplayerActor` _returnvalue))
      (message `/Game/Blueprints/Interfaces/BPI_Displayer.ChangeText` _output_get InText))))

(event `Client_ShowDisplayer`
  (params (TextToShow :type Text) (DisplayerLocation :type "Vector Structure"))
  (bind _existingdisplayer (`self.GetExistingDisplayer`))
  (`/Engine/EditorBlueprintResources/StandardMacros.IsValid` _existingdisplayer
    (:`Is Valid`
      (`Actor.K2_SetActorLocation` _existingdisplayer DisplayerLocation false true)
      (message `/Game/Blueprints/Interfaces/BPI_Displayer.ChangeText` _existingdisplayer TextToShow))
    (:`Is Not Valid`
      (bind _returnvalue (`|SpawnActorFromClass` (`self.DisplayerClass`) (`KismetMathLibrary.MakeTransform` DisplayerLocation) "AlwaysSpawn" "OverrideRootScale" null (`self.ShouldReplicates`) (`GameplayStatics.GetPlayerPawn` 0)))
      (bind _output_get (set `self.DisplayerActor` _returnvalue))
      (message `/Game/Blueprints/Interfaces/BPI_Displayer.ChangeText` _output_get TextToShow))))

(event `ShowDisplayer`
  (params (TextToShow :type Text) (DisplayerLocation :type "Vector Structure"))
  (if (`self.ShouldReplicates`)
    (`self.Server_ShowDisplayer` TextToShow DisplayerLocation)
    (`self.Multi_PlaySound`)
    (else
      (`self.Client_ShowDisplayer` TextToShow DisplayerLocation)
      (`GameplayStatics.PlaySound2D` (`self.SFX`) 1.0 1.0 0.0 null null))))

(event `Server_EditDisplayer`
  (params (TextToShow :type Text))
  (bind _existingdisplayer (`self.GetExistingDisplayer`))
  (`/Engine/EditorBlueprintResources/StandardMacros.IsValid` _existingdisplayer
    (:`Is Valid`
      (message `/Game/Blueprints/Interfaces/BPI_Displayer.ChangeText` _existingdisplayer TextToShow))))

(event `Client_EditDisplayer`
  (params (TextToShow :type Text))
  (bind _existingdisplayer (`self.GetExistingDisplayer`))
  (`/Engine/EditorBlueprintResources/StandardMacros.IsValid` _existingdisplayer
    (:`Is Valid`
      (message `/Game/Blueprints/Interfaces/BPI_Displayer.ChangeText` _existingdisplayer TextToShow))))

(event `EditDisplayer`
  (params (TextToShow :type Text))
  (if (`self.ShouldReplicates`)
    (`self.Server_EditDisplayer` TextToShow)
    (`self.Multi_PlaySound`)
    (else
      (`self.Client_EditDisplayer` TextToShow)
      (`GameplayStatics.PlaySound2D` (`self.SFX`) 1.0 1.0 0.0 null null))))

(event `DeleteDisplayer`
  (if (`self.ShouldReplicates`)
    (`self.Server_DeleteGuide`)
    (else
      (`self.Client_DeleteGuide`))))

(event `Server_DeleteGuide`
  (bind _existingdisplayer (`self.GetExistingDisplayer`))
  (`/Engine/EditorBlueprintResources/StandardMacros.IsValid` _existingdisplayer
    (:`Is Valid`
      (`Actor.K2_DestroyActor` _existingdisplayer))))

(event `Client_DeleteGuide`
  (bind _existingdisplayer (`self.GetExistingDisplayer`))
  (`/Engine/EditorBlueprintResources/StandardMacros.IsValid` _existingdisplayer
    (:`Is Valid`
      (`Actor.K2_DestroyActor` _existingdisplayer))))

(event `Multi_PlaySound`
  (`GameplayStatics.PlaySound2D` (`self.SFX`) 1.0 1.0 0.0 null (`GameplayStatics.GetPlayerController` 0)))

(fn `GetExistingDisplayer`
  (returns (ExistingDisplayer :type "/Game/Blueprints/BP_DisplayerEntity Object Reference"))
  (bind _displayeractor (`self.DisplayerActor`))
  (`/Engine/EditorBlueprintResources/StandardMacros.IsValid` _displayeractor
    (:`Is Valid`
      (return _displayeractor))
    (:`Is Not Valid`
      (bind _returnvalue (`GameplayStatics.GetActorOfClass` (`self.DisplayerClass`)))
      (`/Engine/EditorBlueprintResources/StandardMacros.IsValid` _returnvalue
        (:`Is Valid`
          (return _returnvalue))
        (:`Is Not Valid`
          (return null))))))