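; Actor component that adds proximity-style VOIP voice chat to its owning actor.
; On BeginPlay it creates a VOIP talker, retrying until player state 0 is valid, then registers with it.
; It sets the mic threshold and attaches voice to the owner's root with SA_VoiceChat attenuation.
; Enable, disable and toggle events drive the ToggleSpeaking console command, auto-enabling for locally controlled instigators when IsEnabled is set.
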(event `self.ReceiveBeginPlay`
  (`self.SetupVoiceChat`))

(event `SetupVoiceChat`
  (bind _returnvalue (`|AddComponentByClass` (`self.GetOwner`) "/Script/Engine.VOIPTalker"))
  (set `self.VOIPRef` _returnvalue)
  (`/Engine/EditorBlueprintResources/StandardMacros.IsValid` (`GameplayStatics.GetPlayerState` 0) :!label _label
    (:`Is Valid`
      (`VOIPTalker.RegisterWithPlayerState` (`self.VOIPRef`) (`GameplayStatics.GetPlayerState` 0))
      (`VOIPStatics.SetMicThreshold` -1.0)
      (set `VOIPTalker.Settings` (make `VoiceSettings` (`Actor.RootComponent` (`self.GetOwner`)) "/Game/Woogle/SA_VoiceChat.SA_VoiceChat") (`self.VOIPRef`))
      (if (`Pawn.IsLocallyControlled` (`Actor.Instigator` (`self.GetOwner`)))
        (if (`self.IsEnabled`)
          (`self.EnableVoiceChat`))))
    (:`Is Not Valid`
      (`KismetSystemLibrary.Delay` 0.2)
      (goto _label))))

(event `EnableVoiceChat`
  (`KismetSystemLibrary.ExecuteConsoleCommand` "ToggleSpeaking 1" null)
  (set `self.IsEnabled` true))

(event `ToggleVoiceChat`
  (if (`self.IsEnabled`)
    (`self.DisableVoiceChat`)
    (else
      (`self.EnableVoiceChat`))))

(event `DisableVoiceChat`
  (`KismetSystemLibrary.ExecuteConsoleCommand` "ToggleSpeaking 0" null)
  (set `self.IsEnabled` false))