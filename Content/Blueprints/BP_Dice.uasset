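; Physics-driven six-sided dice actor that throws itself upward on BeginPlay and prints the rolled value.
; RollDice applies an impulse to the Box component, waits RollingTime, then calls CheckDiceValue.
; CheckDiceValue matches actor roll, pitch and yaw against six fixed orientations within five degrees.
; Because yaw must also match, any other resting rotation prints an error and returns -1.
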(event `self.ReceiveBeginPlay`
  (`self.RollDice` (0.0 0.0 1000.0)))

(event `RollDice`
  (params (Impulse :type "Vector Structure"))
  (`PrimitiveComponent.AddImpulse` (`self.Box`) Impulse "None" false)
  (`KismetSystemLibrary.Delay` (`self.RollingTime`))
  (bind _output_get (set `self.DiceValue` (`self.CheckDiceValue`)))
  (`KismetSystemLibrary.PrintString` (`KismetStringLibrary.Concat_StrStr` "Dice Value : " (`KismetStringLibrary.Conv_IntToString` _output_get))))

(fn `CheckDiceValue`
  (returns (Result :type Integer))
  (bind (_returnvalue_roll _returnvalue_pitch _returnvalue_yaw) (`KismetMathLibrary.BreakRotator` (`self.K2_GetActorRotation`)))
  (bind (_returnvalue_roll_2 _returnvalue_pitch_2 _returnvalue_yaw_2) (`KismetMathLibrary.BreakRotator` (`self.K2_GetActorRotation`)))
  (bind (_returnvalue_roll_3 _returnvalue_pitch_3 _returnvalue_yaw_3) (`KismetMathLibrary.BreakRotator` (`self.K2_GetActorRotation`)))
  (bind (_returnvalue_roll_4 _returnvalue_pitch_4 _returnvalue_yaw_4) (`KismetMathLibrary.BreakRotator` (`self.K2_GetActorRotation`)))
  (bind (_returnvalue_roll_5 _returnvalue_pitch_5 _returnvalue_yaw_5) (`KismetMathLibrary.BreakRotator` (`self.K2_GetActorRotation`)))
  (bind (_returnvalue_roll_6 _returnvalue_pitch_6 _returnvalue_yaw_6) (`KismetMathLibrary.BreakRotator` (`self.K2_GetActorRotation`)))
  (if (and (> _returnvalue_roll -5.0) (< _returnvalue_roll 5.0) (> _returnvalue_pitch -95.0) (< _returnvalue_pitch -85.0) (> _returnvalue_yaw -5.0) (< _returnvalue_yaw 5.0))
    (return 1)
    (elif (and (> _returnvalue_roll_2 -95.0) (< _returnvalue_roll_2 -85.0) (> _returnvalue_pitch_2 -5.0) (< _returnvalue_pitch_2 5.0) (> _returnvalue_yaw_2 85.0) (< _returnvalue_yaw_2 95.0))
      (return 2)
      (elif (and (> _returnvalue_roll_3 -5.0) (< _returnvalue_roll_3 5.0) (> _returnvalue_pitch_3 -5.0) (< _returnvalue_pitch_3 5.0) (> _returnvalue_yaw_3 -5.0) (< _returnvalue_yaw_3 5.0))
        (return 3)
        (elif (and (> _returnvalue_roll_4 175.0) (< _returnvalue_roll_4 185.0) (> _returnvalue_pitch_4 -5.0) (< _returnvalue_pitch_4 5.0) (> _returnvalue_yaw_4 175.0) (< _returnvalue_yaw_4 185.0))
          (return 4)
          (elif (and (> _returnvalue_roll_5 85.0) (< _returnvalue_roll_5 95.0) (> _returnvalue_pitch_5 -5.0) (< _returnvalue_pitch_5 5.0) (> _returnvalue_yaw_5 -5.0) (< _returnvalue_yaw_5 5.0))
            (return 5)
            (elif (and (> _returnvalue_roll_6 -5.0) (< _returnvalue_roll_6 5.0) (> _returnvalue_pitch_6 85.0) (< _returnvalue_pitch_6 95.0) (> _returnvalue_yaw_6 -5.0) (< _returnvalue_yaw_6 5.0))
              (return 6)
              (else
                (`KismetSystemLibrary.PrintString` "Dice Error!")
                (return -1)))))))))

(fn `UserConstructionScript`)