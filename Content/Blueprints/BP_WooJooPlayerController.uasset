(event `Key|SpaceBar`
  (params (Key :type "Key Structure"))
  ;[1 1 1] TEST
  (:`Pressed`
    (if (`self.IsMyTurn`)
      (`self.HandleSpaceBar`))))

(event `OnStartBoardGame`
  (if (`self.IsLocalController`)
    (`/Game/Blueprints/BP_DisplayerController.ShowDisplayer` (`self.BP_DisplayerController_Right`) (select `bool` (`self.IsMyTurn`) :`false` "WAITING" :`true` "YOUR TURN" :!type "Text") (`self.GetRightUIPosition`))))

(event `Server_Action`
  (bind _asbp_board_game_mode (cast `/Game/Blueprints/BP_BoardGameMode` (`GameplayStatics.GetGameMode`)))
  (`/Game/Blueprints/BP_BoardGameMode.CycleTurns` _asbp_board_game_mode))

(event `Key|Enter`
  (params (Key :type "Key Structure"))
  ;[1 1 1] TEST
  (:`Pressed`
    (bind _asbp_board_game_mode (cast `/Game/Blueprints/BP_BoardGameMode` (`GameplayStatics.GetGameMode`)))
    (`/Game/Blueprints/BP_BoardGameMode.LetsStart` _asbp_board_game_mode)))

(event `OnStartTurn`
  (`self.SetMyTurn` true)
  (`/Game/Blueprints/BP_DisplayerController.EditDisplayer` (`self.BP_DisplayerController_Right`) "YOUR TURN"))

(event `OnEndTurn`
  (`self.SetMyTurn` false)
  (`/Game/Blueprints/BP_DisplayerController.EditDisplayer` (`self.BP_DisplayerController_Right`) "WAITING"))

(fn `HandleSpaceBar`
  (`self.Server_Action`))

(fn `SetMyTurn`
  (params (IsMyTurn :type Boolean))
  (bind _output_get (set `self.IsMyTurn` IsMyTurn))
  (`self.OnMyTurnChanged` _output_get))

(fn `UserConstructionScript`)