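; BP_DisplayerController manages a single displayer actor that shows a text message in the world.
; ShowDisplayer and DeleteGuide forward to server events that update the existing displayer's text, spawn one at the given location if none exists, or destroy it.
; GetExistingDisplayer prefers the cached actor reference and falls back to searching the world by class, so an existing displayer is reused.
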(event `ShowDisplayer`
  (params (TextToShow :type Text) (DisplayerLocation :type "Vector Structure"))
  (`self.Server_ShowDisplayer` TextToShow DisplayerLocation))

(event `DeleteGuide`
  (`self.Server_DeleteGuide`))

(event `Server_ShowDisplayer`
  (params (InText :type Text) (DisplayerLocation :type "Vector Structure"))
  (bind _existingdisplayer (`self.GetExistingDisplayer`))
  (`/Engine/EditorBlueprintResources/StandardMacros.IsValid` _existingdisplayer
    (:`Is Valid`
      (message `/Game/Blueprints/BPI_Displayer.ChangeText` _existingdisplayer InText))
    (:`Is Not Valid`
      (bind _returnvalue (`|SpawnActorFromClass` (`self.DisplayerClass`) (`KismetMathLibrary.MakeTransform` DisplayerLocation) "AlwaysSpawn" "OverrideRootScale" null (`GameplayStatics.GetPlayerPawn` 0)))
      (bind _output_get (set `self.DisplayerActor` _returnvalue))
      (message `/Game/Blueprints/BPI_Displayer.ChangeText` _output_get InText))))

(event `Server_DeleteGuide`
  (bind _existingdisplayer (`self.GetExistingDisplayer`))
  (`/Engine/EditorBlueprintResources/StandardMacros.IsValid` _existingdisplayer
    (:`Is Valid`
      (`Actor.K2_DestroyActor` _existingdisplayer))))

(fn `GetExistingDisplayer`
  (returns (ExistingDisplayer :type "/Game/Blueprints/BP_DisplayerEntity Object Reference"))
  (bind _displayeractor (`self.DisplayerActor`))
  (`/Engine/EditorBlueprintResources/StandardMacros.IsValid` _displayeractor
    (:`Is Valid`
      (return _displayeractor))
    (:`Is Not Valid`
      (bind _returnvalue (`GameplayStatics.GetActorOfClass` (`self.DisplayerClass`)))
      (`/Engine/EditorBlueprintResources/StandardMacros.IsValid` _returnvalue
        (:`Is Valid`
          (return _returnvalue))
        (:`Is Not Valid`
          (return null))))))