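; Pawn component that sets up spatialized proximity voice chat for its owning player.
; On BeginPlay it adds a VOIPTalker to the pawn and polls on a short delay until the PlayerState cached at startup is valid, without re-reading it.
; It then registers the talker, sets the mic threshold and attaches voice to the root component with SA_VoiceChat attenuation.
; Locally controlled pawns enable speaking through the ToggleSpeaking console command.
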(event `self.ReceiveBeginPlay`
  (set `self.OwnerPawn` (cast `Pawn` (`self.GetOwner`) :!pure true))
  (set `self.OwnerPlayerState` (`Pawn.PlayerState` (`self.OwnerPawn`)))
  (`self.SetupVoiceChat`))

(event `SetupVoiceChat`
  (bind _returnvalue (`|AddComponentByClass` (`self.OwnerPawn`) "/Script/Engine.VOIPTalker"))
  (set `self.VOIPRef` _returnvalue)
  (`/Engine/EditorBlueprintResources/StandardMacros.IsValid` (`self.OwnerPlayerState`) :!label _label
    (:`Is Valid`
      (`VOIPTalker.RegisterWithPlayerState` (`self.VOIPRef`) (`self.OwnerPlayerState`))
      (`VOIPStatics.SetMicThreshold` -1.0)
      (set `VOIPTalker.Settings` (make `VoiceSettings` (`Actor.RootComponent` (`self.OwnerPawn`)) "/Game/Woogle/SA_VoiceChat.SA_VoiceChat") (`self.VOIPRef`))
      (if (`Pawn.IsLocallyControlled` (`self.OwnerPawn`))
        (`KismetSystemLibrary.ExecuteConsoleCommand` "ToggleSpeaking 1" null)))
    (:`Is Not Valid`
      (`KismetSystemLibrary.Delay` 0.2)
      (goto _label))))