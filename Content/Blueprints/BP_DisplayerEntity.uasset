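; Displayer actor that shows a text message through its widget component, starting with DefaultText on BeginPlay when that is not empty.
; ChangeText routes the message to a server or client event according to the ShouldReplicates flag, which the construction script also applies to actor replication.
; Both events pass the text straight to the widget's ChangeTextMessage.
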(event `self.ReceiveBeginPlay`
  (bind _defaulttext (`self.DefaultText`))
  (if (not (`KismetTextLibrary.TextIsEmpty` _defaulttext))
    (`/Game/Blueprints/Interfaces/BPI_Displayer.ChangeText` _defaulttext)))

(event `/Game/Blueprints/Interfaces/BPI_Displayer.ChangeText`
  (params (TextToShow :type Text))
  (if (`self.ShouldReplicates`)
    (`self.Server_ChangeText` TextToShow)
    (else
      (`self.Client_ChangeText` TextToShow))))

(event `Server_ChangeText`
  (params (TextToShow :type Text))
  (message `/Game/Blueprints/Interfaces/BPI_Displayer.ChangeText` (`WidgetComponent.GetUserWidgetObject` (`self.Widget`)) TextToShow))

(event `Client_ChangeText`
  (params (TextToShow :type Text))
  (message `/Game/Blueprints/Interfaces/BPI_Displayer.ChangeText` (`WidgetComponent.GetUserWidgetObject` (`self.Widget`)) TextToShow))

(fn `UserConstructionScript`
  (`self.SetReplicates` (`self.ShouldReplicates`)))