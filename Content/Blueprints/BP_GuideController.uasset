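; BP_GuideController shows and removes an in-world text guide sign, represented by a BP_GuideDisplayer actor.
; Public DisplayGuide and DeleteGuide events forward to server-named events, which update, spawn or destroy the sign.
; GetExistingGuideSign checks the cached reference, then searches the world for any displayer, so an existing sign is reused instead of duplicated.
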(event `DisplayGuide`
  (params (InText :type Text))
  (`self.Server_DisplayGuide` InText))

(event `DeleteGuide`
  (`self.Server_DeleteGuide`))

(event `Server_DisplayGuide`
  (params (InText :type Text))
  (bind _existingguidesign (`self.GetExistingGuideSign`))
  (`/Engine/EditorBlueprintResources/StandardMacros.IsValid` _existingguidesign
    (:`Is Valid`
      (`/Game/Blueprints/BP_GuideDisplayer.ChangeText` _existingguidesign InText))
    (:`Is Not Valid`
      (bind _returnvalue (`|SpawnActorFromClass` "/Game/Blueprints/BP_GuideDisplayer.BP_GuideDisplayer_C" (`KismetMathLibrary.MakeTransform` (`self.SpawnLocation`)) "AlwaysSpawn" "OverrideRootScale" null (`GameplayStatics.GetPlayerPawn` 0)))
      (bind _output_get (set `self.GuideDisplayer` _returnvalue))
      (`/Game/Blueprints/BP_GuideDisplayer.ChangeText` _output_get InText))))

(event `Server_DeleteGuide`
  (bind _existingguidesign (`self.GetExistingGuideSign`))
  (`/Engine/EditorBlueprintResources/StandardMacros.IsValid` _existingguidesign
    (:`Is Valid`
      (`Actor.K2_DestroyActor` _existingguidesign))))

(fn `GetExistingGuideSign`
  (returns (ExistingGuideSign :type "/Game/Blueprints/BP_GuideDisplayer Object Reference"))
  (bind _guidedisplayer (`self.GuideDisplayer`))
  (`/Engine/EditorBlueprintResources/StandardMacros.IsValid` _guidedisplayer
    (:`Is Valid`
      (return _guidedisplayer))
    (:`Is Not Valid`
      (bind _returnvalue (`GameplayStatics.GetActorOfClass` "/Game/Blueprints/BP_GuideDisplayer.BP_GuideDisplayer_C"))
      (`/Engine/EditorBlueprintResources/StandardMacros.IsValid` _returnvalue
        (:`Is Valid`
          (return _returnvalue))
        (:`Is Not Valid`
          (return null))))))